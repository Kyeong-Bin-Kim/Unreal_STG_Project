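; Boss map tile for the STG project that starts the boss encounter and spawns the mosquito enemy.
; On BeginPlay it calls CallBossMeeting, which is not defined in this graph, then spawns BP_Mosquito at the fifth spawn area with a fixed rotation.
; The mosquito is attached to the tile with keep-world rules.
; The construction script collects the nine spawn area components into SpawnBoxes, though the boss spawn references its area directly.
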(event `self.ReceiveBeginPlay`
  (`self.BossMeeting`)
  (`self.SpawnBossEnemy`))

(event `SpawnBossEnemy`
  (bind _returnvalue (`|SpawnActorFromClass` "/Game/STG_Project/BluePrint/Enemy/BP_Mosquito.BP_Mosquito_C" (`KismetMathLibrary.MakeTransform` (`SceneComponent.K2_GetComponentLocation` (`self.EnemySpownArea5`)) (struct :`Yaw` 90.0)) "Undefined" "MultiplyWithRoot" self null))
  (`self.K2_AttachToActor` _returnvalue self "None" "KeepWorld" "KeepWorld" "KeepWorld" false))

(fn `UserConstructionScript`
  (set `self.SpawnBoxes` (`|MakeArray` (`self.EnemySpownArea1`) (`self.EnemySpownArea2`) (`self.EnemySpownArea3`) (`self.EnemySpownArea4`) (`self.EnemySpownArea5`) (`self.EnemySpownArea6`) (`self.EnemySpownArea7`) (`self.EnemySpownArea8`) (`self.EnemySpownArea9`))))