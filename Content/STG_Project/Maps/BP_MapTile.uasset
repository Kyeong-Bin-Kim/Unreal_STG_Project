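; BP_MapTile is a map tile that populates itself with enemies and triggers spawning of the next tile.
; On BeginPlay it caches BP_MapManager, then picks a random set of unique locations from nine spawn areas gathered in the construction script.
; It spawns a BP_Beholder at each location and attaches it to the tile.
; When a BP_SwarmPlayer overlaps PlayerSensor, it calls SpawnTile on the map manager.
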(event `self.ReceiveBeginPlay`
  (bind _outactors (`GameplayStatics.GetAllActorsOfClass` "/Game/STG_Project/Maps/BP_MapManager.BP_MapManager_C"))
  (set `self.MapManagerReference` (`|GetArrayItem` _outactors))
  (`self.SpawnAddLocation`)
  (`self.SpawnEnemy`))

(event `SpawnAddLocation`
  (`KismetArrayLibrary.Array_Clear` (`self.SpawnedLocations`))
  (for _ (range (+ (`KismetMathLibrary.RandomIntegerInRange` 1 7) 1))
    (`KismetArrayLibrary.Array_AddUnique` (`self.SpawnedLocations`) (`SceneComponent.K2_GetComponentLocation` (`KismetArrayLibrary.Array_Random` (`self.SpawnBoxes`))))))

(event `SpawnEnemy`
  (for _index (range (`KismetArrayLibrary.Array_Length` (`self.SpawnedLocations`)))
    (bind _returnvalue (`|SpawnActorFromClass` "/Game/STG_Project/BluePrint/Enemy/BP_Beholder.BP_Beholder_C" (`KismetMathLibrary.MakeTransform` (`|GetArrayItem` (`self.SpawnedLocations`) _index) (struct :`Yaw` 180.0)) "Undefined" "MultiplyWithRoot" self null))
    (`self.K2_AttachToActor` _returnvalue self "None" "KeepWorld" "KeepWorld" "KeepWorld" false)))

(event `self.PlayerSensor.OnComponentBeginOverlap`
  (params (OverlappedComponent :type "PrimitiveComponent Object Reference") (OtherActor :type "Actor Object Reference") (OtherComp :type "PrimitiveComponent Object Reference") (OtherBodyIndex :type Integer) (bFromSweep :type Boolean) (SweepResult :type "HitResult Structure (by ref)"))
  (cast `/Game/STG_Project/BluePrint/Character/BP_SwarmPlayer` OtherActor)
  (if (`PrimitiveComponent.IsOverlappingActor` (`self.PlayerSensor`) OtherActor)
    (`/Game/STG_Project/Maps/BP_MapManager.SpawnTile` (`self.MapManagerReference`))))

(fn `UserConstructionScript`
  (set `self.SpawnBoxes` (`|MakeArray` (`self.EnemySpownArea1`) (`self.EnemySpownArea2`) (`self.EnemySpownArea3`) (`self.EnemySpownArea4`) (`self.EnemySpownArea5`) (`self.EnemySpownArea6`) (`self.EnemySpownArea7`) (`self.EnemySpownArea8`) (`self.EnemySpownArea9`))))