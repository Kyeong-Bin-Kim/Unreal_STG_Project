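; Mosquito enemy for the boss map that fires projectiles, teleports between spawn areas and explodes in a Niagara effect when its health runs out.
; A looping timer started after BeginPlay drives attacks, keeping the attack montage playing while spawning projectiles.
; Every tenth attack switches it to a delayed jump to a random location.
; The construction script gathers those locations from the first BP_BossMapTile and fills the array of spawn arrows.
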(event `self.ReceiveAnyDamage`
  (params (Damage :type "Float (single-precision)") (DamageType :type "DamageType Object Reference") (InstigatedBy :type "Controller Object Reference") (DamageCauser :type "Actor Object Reference"))
  (bind _output_get (set `self.Hp` (- (`self.Hp`) Damage)))
  (if (<= _output_get 0.0)
    (`self.OnDie`)))

(event `/Game/STG_Project/Interface/BPI_Die.OnDie`
  (`NiagaraFunctionLibrary.SpawnSystemAtLocation` (`self.DieExplosion`) (`self.K2_GetActorLocation`) (struct) (1.0 1.0 1.0) true true "AutoRelease")
  (`self.K2_DestroyActor`))

(event `self.ReceiveBeginPlay`
  (`KismetSystemLibrary.Delay` 2.0)
  (`KismetSystemLibrary.K2_SetTimerDelegate` (delegate `/Game/STG_Project/Interface/BPI_Attack.Attack`) (`self.AttackInterval`) true))

(event `/Game/STG_Project/Interface/BPI_Attack.Attack`
  (bind _attackmontage (`self.AttackMontage`))
  (bind _returnvalue (`SkeletalMeshComponent.GetAnimInstance` (`self.SkeletalMesh`)))
  (if (`self.IsAttacking`)
    (`KismetSystemLibrary.Delay` 3.0)
    (`self.MoveToTarget`)
    (set `self.IsAttacking` false)
    (else
      (`/Engine/EditorBlueprintResources/StandardMacros.IncrementInt` (`self.AttackCount`)
        (:`  `
          (if (`AnimInstance.Montage_IsPlaying` _returnvalue _attackmontage)
            (if (not (`self.IsAttacking`))
              (if (== (mod (`self.AttackCount`) 10) 0) :!label _label
                (set `self.IsAttacking` true))
              (`|SpawnActorFromClass` (`self.GetProjectileClass`) (`self.GetAttackProjectileLocation`) "Undefined" "MultiplyWithRoot" null null))
            (else
              (`AnimInstance.Montage_Play` _returnvalue _attackmontage 1.0 "MontageLength" 0.0 true)
              (goto _label))))))))

(event `MoveToTarget`
  (bind _outitem (`KismetArrayLibrary.Array_Random` (`self.TargetLocation`)))
  (if (!= (`SceneComponent.K2_GetComponentLocation` (`self.SkeletalMesh`)) _outitem)
    (`self.K2_SetActorLocation` _outitem)))

(fn `UserConstructionScript`
  (bind _output (`|GetArrayItem` (`self.TileLocation`)))
  (`KismetArrayLibrary.Array_Clear` (`self.AttackSpawnArrow`))
  (set `self.AttackSpawnArrow` (`|MakeArray` (`self.Arrow1`) (`self.Arrow2`) (`self.Arrow3`) (`self.Arrow4`) (`self.Arrow5`) (`self.Arrow6`) (`self.Arrow7`) (`self.Arrow8`) (`self.Arrow9`)))
  (`KismetArrayLibrary.Array_Clear` (`self.TileLocation`))
  (bind _outactors (`GameplayStatics.GetAllActorsOfClass` "/Game/STG_Project/Maps/BP_BossMapTile.BP_BossMapTile_C"))
  (set `self.TileLocation` _outactors)
  (`KismetArrayLibrary.Array_Clear` (`self.TargetLocation`))
  (set `self.TargetLocation` (`|MakeArray` (`SceneComponent.K2_GetComponentLocation` (`/Game/STG_Project/Maps/BP_BossMapTile.EnemySpownArea1` _output)) (`SceneComponent.K2_GetComponentLocation` (`/Game/STG_Project/Maps/BP_BossMapTile.EnemySpownArea2` _output)) (`SceneComponent.K2_GetComponentLocation` (`/Game/STG_Project/Maps/BP_BossMapTile.EnemySpownArea3` _output)) (`SceneComponent.K2_GetComponentLocation` (`/Game/STG_Project/Maps/BP_BossMapTile.EnemySpownArea4` _output)) (`SceneComponent.K2_GetComponentLocation` (`/Game/STG_Project/Maps/BP_BossMapTile.EnemySpownArea5` _output)) (`SceneComponent.K2_GetComponentLocation` (`/Game/STG_Project/Maps/BP_BossMapTile.EnemySpownArea6` _output)) (`SceneComponent.K2_GetComponentLocation` (`/Game/STG_Project/Maps/BP_BossMapTile.EnemySpownArea7` _output)) (`SceneComponent.K2_GetComponentLocation` (`/Game/STG_Project/Maps/BP_BossMapTile.EnemySpownArea8` _output)) (`SceneComponent.K2_GetComponentLocation` (`/Game/STG_Project/Maps/BP_BossMapTile.EnemySpownArea9` _output)))))