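; Player controller that handles player death and level restart for the swarm player pawn.
; On possess, it binds to the BP_SwarmPlayer death event, whose handler removes and immediately re-adds the same IMC_Player mapping context.
; The restart input action resets player HP on the GI_PlayerHP game instance and reopens the play level.
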(event `self.ReceivePossess`
  (params (PossessedPawn :type "Pawn Object Reference"))
  (bind _asbp_swarm_player (cast `/Game/STG_Project/BluePrint/Character/BP_SwarmPlayer` PossessedPawn))
  (add `/Game/STG_Project/BluePrint/Character/BP_SwarmPlayer.OnDie` _asbp_swarm_player (delegate `OnPlayerDie`)))

(event `OnPlayerDie`
  (bind _returnvalue (subsystem `EnhancedInputLocalPlayerSubsystem`))
  (`EnhancedInputSubsystemInterface.RemoveMappingContext` _returnvalue "/Game/STG_Project/Input/IMC_Player.IMC_Player" (struct))
  (`EnhancedInputSubsystemInterface.AddMappingContext` _returnvalue "/Game/STG_Project/Input/IMC_Player.IMC_Player" 0 (struct)))

(event `EnhancedInput|/Game/STG_Project/Input/IA_PlayerRestart`
  (params (ActionValue :type "Vector2D Structure") (ElapsedSeconds :type "Float (double-precision)") (TriggeredSeconds :type "Float (double-precision)") (InputAction :type "InputAction Object Reference" :default "/Game/STG_Project/Input/IA_PlayerRestart.IA_PlayerRestart"))
  (:`Triggered`
    (bind _asgi_player_hp (cast `/Game/STG_Project/BluePrint/Framework/GI_PlayerHP` (`GameplayStatics.GetGameInstance`)))
    (set `/Game/STG_Project/BluePrint/Framework/GI_PlayerHP.PlayerHp` 3.0 _asgi_player_hp)
    (`GameplayStatics.OpenLevelBySoftObjectPtr` (`self.PlayLevel`))))

(fn `UserConstructionScript`)