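; BP_PlayerProjectile is a player projectile that damages what it overlaps and explodes.
; Overlapping any actor not tagged Player or Bullet applies damage, then calls the Destroy event, which a lifetime timer started at BeginPlay also triggers.
; Destroy spawns an auto-release pooled explosion effect at the projectile's location, resets its location and rotation, then destroys the actor.
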(event `self.ReceiveBeginPlay`
  (`KismetSystemLibrary.K2_SetTimerDelegate` (delegate `Destroy`) (`self.LifeTime`)))

(event `Destroy`
  (`NiagaraFunctionLibrary.SpawnSystemAtLocation` (`self.ExplosionEffect`) (`self.K2_GetActorLocation`) (struct) (1.0 1.0 1.0) true true "AutoRelease")
  (`self.K2_SetActorLocationAndRotation` (0.0 0.0 0.0))
  (`self.K2_DestroyActor`))

(event `self.ReceiveActorBeginOverlap`
  (params (OtherActor :type "Actor Object Reference"))
  (if (not (or (`self.ActorHasTag` OtherActor "Player") (`self.ActorHasTag` OtherActor "Bullet")))
    (`GameplayStatics.ApplyDamage` OtherActor (`self.Damage`))
    (`self.Destroy`)))

(fn `UserConstructionScript`)