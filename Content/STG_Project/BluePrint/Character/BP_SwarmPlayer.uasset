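; BP_SwarmPlayer is the player-controlled flyer, which moves constantly along world +X and fires projectiles.
; Enhanced Input sets lateral and vertical vectors that FlyingSystem applies each Tick as movement input, climbing while Space is held and descending otherwise.
; Attack plays a montage, spawns a projectile at the AttackSoket socket, and blocks re-firing for the montage's length.
; Current HP starts at MaxHp, with no damage handling here.
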(event `self.ReceiveBeginPlay`
  (`EnhancedInputSubsystemInterface.AddMappingContext` (pcsubsystem `EnhancedInputLocalPlayerSubsystem` (`GameplayStatics.GetPlayerController` 0)) "/Game/STG_Project/Input/IMC_Player.IMC_Player" 0 (struct))
  (set `self.CurrenHp` (`self.MaxHp`)))

(event `self.ReceiveTick`
  (params (DeltaSeconds :type "Float (single-precision)"))
  (if (not (`self.IsKeyInputCheck`))
    (set `self.MoveVectorZ` (0.0 0.0 -1.0))
    (set `self.IsKeyInputCheck` true))
  (`self.AddMovementInput` (1.0 0.0 0.0) (* DeltaSeconds (`self.MoveSpeed`)))
  (if (`self.IsAscending`)
    (`self.AddMovementInput` (+ (`self.MoveVectorX`) (`self.MoveVectorZ`)) (* DeltaSeconds (`self.MoveSpeed`)))
    (else
      (`self.AddMovementInput` (+ (`self.MoveVectorX`) (`self.MoveVectorZ`)) (* DeltaSeconds (`self.MoveSpeed`))))))

(event `EnhancedInput|/Game/STG_Project/Input/IA_PlayerMove`
  (params (ActionValue :type "Vector2D Structure") (ElapsedSeconds :type "Float (double-precision)") (TriggeredSeconds :type "Float (double-precision)") (InputAction :type "InputAction Object Reference" :default "/Game/STG_Project/Input/IA_PlayerMove.IA_PlayerMove"))
  (:`Triggered`
    (set `self.IsKeyInputCheck` true)
    (set `self.MoveVectorX` (* (`KismetMathLibrary.BreakVector2D` ActionValue) (`self.GetActorRightVector`))))
  (:`Completed`
    (set `self.MoveVectorX` (0.0 0.0 0.0))))

(event `EnhancedInput|/Game/STG_Project/Input/IA_Player_Space`
  (params (ActionValue :type Boolean) (ElapsedSeconds :type "Float (double-precision)") (TriggeredSeconds :type "Float (double-precision)") (InputAction :type "InputAction Object Reference" :default "/Game/STG_Project/Input/IA_Player_Space.IA_Player_Space"))
  (:`Started`
    (set `self.IsKeyInputCheck` true)
    (set `self.IsAscending` true)
    (set `self.MoveVectorZ` (`KismetMathLibrary.MakeVector` 0.0 0.0 1.0)))
  (:`Completed`
    (set `self.IsAscending` false)
    (set `self.MoveVectorZ` (`KismetMathLibrary.MakeVector` 0.0 0.0 -1.0))))

(event `EnhancedInput|/Game/STG_Project/Input/IA_PlayerAttack`
  (params (ActionValue :type Boolean) (ElapsedSeconds :type "Float (double-precision)") (TriggeredSeconds :type "Float (double-precision)") (InputAction :type "InputAction Object Reference" :default "/Game/STG_Project/Input/IA_PlayerAttack.IA_PlayerAttack"))
  (:`Started`
    (`self.Attack`)))

(event `/Game/STG_Project/Interface/BPI_Attack.Attack`
  (if (not (`self.IsAttacking`))
    (set `self.IsAttacking` true)
    (bind _returnvalue (`AnimInstance.Montage_Play` (`SkeletalMeshComponent.GetAnimInstance` (`self.SkeletalMesh`)) (`self.AttackMontage`) 1.0 "MontageLength" 0.0 true))
    (bind _attacktransform (`self.GetAttackProjectile`))
    (`|SpawnActorFromClass` (`self.GetProjectileClass`) _attacktransform "Undefined" "MultiplyWithRoot" null null)
    (`KismetSystemLibrary.Delay` _returnvalue)
    (set `self.IsAttacking` false)))

(fn `GetAttackProjectile`
  (returns (AttackTransform :type "Transform Structure"))
  (return (`SceneComponent.GetSocketTransform` (`self.SkeletalMesh`) "AttackSoket" "RTS_World")))

(fn `UserConstructionScript`)